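; BP_Marla is a merchant character that opens a trade UI on interact and periodically restocks its inventory.
; Interacting creates WBP_Trade once, then flip-flops the trade and bag widgets and switches input mode.
; LoadInventory rebuilds the bag list with WBP_Resource widgets from the Inventory map, provided UIBagRef, set outside these graphs, is valid.
; A Delay on Tick acts as a restock timer, incrementing an existing item's count and refreshing the list.
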(event `/Game/005_QuestSystem/Blueprints/BPI/BP_BPI_Interaction.OnInteract`
  (params (PlayerActor :type "Actor Object Reference"))
  (bind _returnvalue (`GameplayStatics.GetPlayerController` 0))
  (bind _ui_trade_ref (`self.UI Trade Ref`))
  (set `PlayerController.bShowMouseCursor` true _returnvalue)
  (`WidgetBlueprintLibrary.SetInputMode_GameAndUIEx` _returnvalue null)
  (`/Engine/EditorBlueprintResources/StandardMacros.IsValid` (`self.UI Trade Ref`)
    (:`Is Valid`
      (`/Engine/EditorBlueprintResources/StandardMacros.FlipFlop`
        (:`A`
          (`Widget.RemoveFromParent` _ui_trade_ref)
          (`Widget.RemoveFromParent` (`self.UI Bag Ref`))
          (set `PlayerController.bShowMouseCursor` false _returnvalue)
          (`WidgetBlueprintLibrary.SetInputMode_GameOnly` _returnvalue))
        (:`B`
          (`UserWidget.AddToViewport` _ui_trade_ref 0)
          (`UserWidget.AddToViewport` (`self.UI Bag Ref`) 0)
          (`self.LoadInventory`))))
    (:`Is Not Valid`
      (bind _returnvalue_2 (`|CreateWidget` "/Game/001_UI/Game/HUD_Trade/WBP_Trade.WBP_Trade_C"))
      (bind _output_get (set `self.UI Trade Ref` _returnvalue_2))
      (`UserWidget.AddToViewport` _output_get 0)
      (`self.LoadInventory`))))

(event `self.ReceiveTick`
  (params (DeltaSeconds :type "Float (single-precision)"))
  (`KismetSystemLibrary.Delay` 180.0)
  (`self.AddItem` 1))

(fn `AddItem`
  (params (ItemIndex :type Integer))
  (bind _inventory (`self.Inventory`))
  (bind (_value _returnvalue) (`BlueprintMapLibrary.Map_Find` _inventory ItemIndex))
  (if _returnvalue
    (bind _structout (setmembers `/Game/004_DataBase/S_Resource` :`StructRef` _value :`Count` (+ (`.Count_51_FDA1585A4C93517474931FA863FE5894` (break `/Game/004_DataBase/S_Resource` _value)) 1)))
    (`BlueprintMapLibrary.Map_Add` _inventory ItemIndex _structout)
    (`self.LoadInventory`)))

(fn `LoadInventory`
  (bind _ui_bag_ref (`self.UI Bag Ref`))
  (`/Engine/EditorBlueprintResources/StandardMacros.IsValid` _ui_bag_ref
    (:`Is Valid`
      (`PanelWidget.ClearChildren` (`/Game/001_UI/Game/HUD_Inventory/WBP_Bag_PNJ.VerticalBoxBag` _ui_bag_ref))
      (bind _values (`BlueprintMapLibrary.Map_Values` (`self.Inventory`)))
      (for _array_element _values
        (bind _returnvalue (`|CreateWidget` "/Game/001_UI/Game/HUD_Inventory/WBP_Resource.WBP_Resource_C" null _array_element))
        (`VerticalBox.AddChildToVerticalBox` (`/Game/001_UI/Game/HUD_Inventory/WBP_Bag_PNJ.VerticalBoxBag` (`self.UI Bag Ref`)) _returnvalue)))))

(fn `UserConstructionScript`)