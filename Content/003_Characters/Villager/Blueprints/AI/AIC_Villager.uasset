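; AIC_Villager is the AI controller for villager characters that sets them up to follow an assigned path.
; On BeginPlay it runs BT_Villager and casts the controlled pawn to BP_Villager.
; It then writes the villager's PathToFollow into the blackboard and seeds the new destination with the world location of that path spline's first point.
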(event `self.ReceiveBeginPlay`
  (`self.RunBehaviorTree` "/Game/003_Characters/Villager/Blueprints/AI/BT_Villager.BT_Villager")
  (bind _asbp_villager (cast `/Game/003_Characters/Villager/Blueprints/BP_Villager` (`self.K2_GetPawn`)))
  (bind _pathtofollow (`/Game/003_Characters/Villager/Blueprints/BP_Villager.PathToFollow` _asbp_villager))
  (`BlackboardComponent.SetValueAsObject` (`self.Blackboard`) (`self.KeyPathToFollow`) _pathtofollow)
  (`BlackboardComponent.SetValueAsVector` (`self.Blackboard`) (`self.KeyNewDestination`) (`SplineComponent.GetLocationAtSplinePoint` (`/Game/003_Characters/Krab/Blueprints/AI/BP_Root.Spline` _pathtofollow) 0 "World")))

(fn `UserConstructionScript`)