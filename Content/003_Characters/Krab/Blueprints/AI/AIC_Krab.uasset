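; AIC_Krab is the AI controller for the Krab character, running the BT_Krab behavior tree on BeginPlay.
; It seeds the blackboard with the pawn's patrol path and the first point of that path's spline as the initial destination.
; AI perception updates the blackboard: heard stimuli store a last known position, while any other sense sets the sensed actor as the player target and clears it when lost.
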(event `self.ReceiveBeginPlay`
  (`self.RunBehaviorTree` "/Game/003_Characters/Krab/Blueprints/AI/BT_Krab.BT_Krab")
  (bind _asbp_krab (cast `/Game/003_Characters/Krab/Blueprints/BP_Krab` (`self.K2_GetPawn`)))
  (bind _pathtofollow (`/Game/003_Characters/Krab/Blueprints/BP_Krab.PathToFollow` _asbp_krab))
  (`BlackboardComponent.SetValueAsObject` (`self.Blackboard`) (`self.KeyPathToFollow`) _pathtofollow)
  (`BlackboardComponent.SetValueAsVector` (`self.Blackboard`) (`self.KeyNewDestination`) (`SplineComponent.GetLocationAtSplinePoint` (`/Game/003_Characters/Krab/Blueprints/AI/BP_Root.Spline` _pathtofollow) 0 "World")))

(event `self.AIPerception.OnTargetPerceptionUpdated`
  (params (Actor :type "Actor Object Reference") (Stimulus :type "AIStimulus Structure"))
  (bind ((`StimulusLocation` _stimuluslocation) (`bSuccessfullySensed` _bsuccessfullysensed)) (break `AIStimulus` (`self.Stimulus`)))
  (set `self.DetectedActor` Actor)
  (bind _output_get (set `self.Stimulus` Stimulus))
  (bind _returnvalue (`AIPerceptionSystem.GetSenseClassForStimulus` _output_get))
  (if (== _returnvalue "/Script/AIModule.AISense_Hearing")
    (if _bsuccessfullysensed
      (`BlackboardComponent.SetValueAsVector` (`self.Blackboard`) (`self.KeyLastPosition`) _stimuluslocation))
    (elif (`.bSuccessfullySensed` (break `AIStimulus` (`self.Stimulus`)))
      (`BlackboardComponent.SetValueAsObject` (`self.Blackboard`) (`self.KeyPlayer`) (`self.DetectedActor`))
      (else
        (`BlackboardComponent.ClearValue` (`self.Blackboard`) (`self.KeyPlayer`))))))

(fn `UserConstructionScript`)