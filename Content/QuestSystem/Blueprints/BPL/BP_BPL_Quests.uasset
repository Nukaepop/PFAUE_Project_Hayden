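; Blueprint function library with shared helpers for the quest system.
; GetQuestComponent looks up the quest component on player character 0 and returns it with a flag saying whether it was found.
; IsValidQuest checks that a quest info struct has an ID and name other than "None" and at least one objective.
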(fn `GetQuestComponent`
  (returns (`ComponentWasFound?` :type Boolean) (QuestComponent :type "/Game/QuestSystem/Blueprints/BP_BPC_PlayerQuestComponent Object Reference"))
  (bind _returnvalue (`Actor.GetComponentByClass` (`GameplayStatics.GetPlayerCharacter` null) "/Game/QuestSystem/Blueprints/BP_BPC_PlayerQuestComponent.BP_BPC_PlayerQuestComponent_C"))
  (`/Engine/EditorBlueprintResources/StandardMacros.IsValid` _returnvalue
    (:`Is Valid`
      (return true _returnvalue))
    (:`Is Not Valid`
      (return false null))))

(fn `IsValidQuest?`
  (params (ST_Quest_Info :type "/Game/QuestSystem/Blueprints/Structures/ST_Quest_Info Structure (by ref)"))
  (returns (`Valid?` :type Boolean))
  (bind ((`QuestID_2_E9DD1B8B405D0E58BEEA3AA29273D9A7` _questid) (`QuestName_5_907584914A22F95110512DB3B6EC1EFB` _questname) (`Objectives_21_50C63F1D4C80B7AA25F0B7B40D0F2E3D` _objectives)) (break `/Game/QuestSystem/Blueprints/Structures/ST_Quest_Info` ST_Quest_Info))
  (return (and (!= _questid "None") (`KismetTextLibrary.NotEqual_TextText` _questname "None") (> (`KismetArrayLibrary.Array_Length` _objectives) 0))))